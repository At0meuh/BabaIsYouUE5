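; BP_Player is a player that moves in discrete steps across a referenced procedural grid, registering IMC_Default on BeginPlay.
; IA_move bounds-checks the target cell against the grid size (inclusive), updates X/Y coordinates, then offsets the actor by CalculLocatonToAdd.
; That function holds a vector calculation from mesh bounds and grid spacing, shown as unused.
; Tick prints current coordinates and grid size for debugging.
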(event `self.ReceiveBeginPlay`
  (bind _asbp_custom_player_controller (cast `/Game/Blueprint/BP_CustomPlayerController` (`self.GetController`)))
  (`EnhancedInputSubsystemInterface.AddMappingContext` (pcsubsystem `EnhancedInputLocalPlayerSubsystem` _asbp_custom_player_controller) "/Game/Input/IMC_Default.IMC_Default" 0 (struct)))

(event `self.ReceiveTick`
  (params (DeltaSeconds :type "Float (single-precision)"))
  (bind _proceduralgridref (`self.ProceduralGridRef`))
  (`KismetSystemLibrary.PrintString` (`KismetStringLibrary.Concat_StrStr` "x : " (`KismetStringLibrary.Conv_IntToString` (`self.XGridCoords`)) " y : " (`KismetStringLibrary.Conv_IntToString` (`self.YGridCoords`))) true true (struct :`G` 0.66 :`B` 1.0 :`A` 1.0) 0.0)
  (`KismetSystemLibrary.PrintString` (`KismetStringLibrary.Concat_StrStr` "x : " (`KismetStringLibrary.Conv_IntToString` (`/Game/Blueprint/BP_proceduralGrid.GridSizeX` _proceduralgridref)) " y : " (`KismetStringLibrary.Conv_IntToString` (`/Game/Blueprint/BP_proceduralGrid.GridSizeY` _proceduralgridref))) true true (struct :`R` 0.931853 :`G` 1.0 :`A` 1.0) 0.0))

(event `EnhancedInput|/Game/Input/Action/IA_move`
  (params (ActionValue :type "Vector2D Structure") (ElapsedSeconds :type "Float (double-precision)") (TriggeredSeconds :type "Float (double-precision)") (InputAction :type "InputAction Object Reference" :default "/Game/Input/Action/IA_move.IA_move"))
  (bind (_x _y) (`KismetMathLibrary.BreakVector2D` ActionValue))
  (bind _proceduralgridref (`self.ProceduralGridRef`))
  (bind _returnvalue (+ (`self.YGridCoords`) (`KismetMathLibrary.FTrunc` _y)))
  (bind _returnvalue_2 (+ (`self.XGridCoords`) (`KismetMathLibrary.FTrunc` _x)))
  (bind (_min _max) (break `Box` (`StaticMesh.GetBoundingBox` (`/Game/Blueprint/BP_proceduralGrid.GridMesh` _proceduralgridref))))
  (bind _x_2 (.x (- _max _min)))
  (bind _y_2 (.y (- _max _min)))
  (:`Started`
    (if (and (<= _returnvalue_2 (`/Game/Blueprint/BP_proceduralGrid.GridSizeX` (`self.ProceduralGridRef`))) (<= _returnvalue (`/Game/Blueprint/BP_proceduralGrid.GridSizeY` (`self.ProceduralGridRef`))) (>= _returnvalue 0) (>= _returnvalue_2 0))
      (set `self.XGridCoords` _returnvalue_2)
      (set `self.YGridCoords` _returnvalue)
      (`self.K2_AddActorWorldOffset` (`KismetMathLibrary.MakeVector` (* _x (+ _x_2 (* _x_2 (`/Game/Blueprint/BP_proceduralGrid.DistanceX` _proceduralgridref)))) (* _y (+ _y_2 (* _y_2 (`/Game/Blueprint/BP_proceduralGrid.DistanceY` _proceduralgridref)))))))))

(fn `UserConstructionScript`)