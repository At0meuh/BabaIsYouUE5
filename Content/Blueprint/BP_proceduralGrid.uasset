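; BP_proceduralGrid builds a flat grid of copies of one configurable mesh and material in its Construction Script.
; Nested loops over GridSizeX and GridSizeY add a separate Static Mesh Component for each cell.
; Each is positioned on local X and Y by the mesh's bounds size, with DistanceX and DistanceY adding gaps as multiples of that size.
; The event graph holds no runtime logic.
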(fn `UserConstructionScript`
  (for _index (range (+ (`self.GridSizeX`) 1))
    (for _index_2 (range (+ (`self.GridSizeY`) 1))
      (bind _returnvalue (`AddComponent|NODE_AddStaticMeshComponent-0`))
      (`StaticMeshComponent.SetStaticMesh` _returnvalue (`self.GridMesh`))
      (`PrimitiveComponent.SetMaterial` _returnvalue 0 (`self.Material`))
      (bind (_min _max) (`StaticMeshComponent.GetLocalBounds` _returnvalue))
      (bind _x (.x (- _max _min)))
      (bind _y (.y (- _max _min)))
      (`SceneComponent.K2_SetRelativeLocation` _returnvalue (`KismetMathLibrary.MakeVector` (+ (* _index _x) (* _x (`self.DistanceX`) _index)) (+ (* _index_2 _y) (* _y (`self.DistanceY`) _index_2))) false false))))